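; Bowling pre-hit trigger that plays a multi-pin sound cue when a pickup sphere enters it while the bowling system awaits the first throw.
; On BeginPlay it looks up the scoring_system actor by name and caches it as the bowling system.
; On overlap it filters for pickup spheres, checks the throw state, then plays the cue at the sphere's location with random pitch and an offset start time.
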(event `self.ReceiveBeginPlay`
  ;[1 1 1] Get reference to Bowling System
  (bind _returnvalue (`entity_base.FindActorByName` "scoring_system" self))
  (bind _asbowling_system_bp (cast `/Game/blueprint/Bowling/bowling_system_BP` _returnvalue))
  (set `self.BowlingSystem` _asbowling_system_bp))

(event `self.ReceiveActorBeginOverlap`
  (params (OtherActor :type "Actor Object Reference"))
  (bind _asbp_pickup_sphere (cast `/Game/blueprint/BP_Pickup_Sphere` OtherActor))
  (if (`bowling_system.WaitingForFirstThrow` (`self.BowlingSystem`))
    (`GameplayStatics.PlaySoundAtLocation` "/Game/sound/bowling/Pin_Lots_Cue.Pin_Lots_Cue" (`self.K2_GetActorLocation` _asbp_pickup_sphere) (struct) 0.6 (`KismetMathLibrary.RandomFloatInRange` 0.8 1.2) 0.9)))

(fn `UserConstructionScript`)