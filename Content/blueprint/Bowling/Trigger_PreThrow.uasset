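; Bowling trigger volume that plays a rolling sound and assists the spin of a thrown pickup ball.
; On overlap it sets timers from ball speed to end the spin assist and trigger a brief global slow motion shortly before that.
; While active, Tick fires a named rotation-helper launcher, with angular speed rising quadratically as the ball nears the highest-velocity target point.
; An autoaim launcher is cached but unused here.
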(event `self.ReceiveBeginPlay`
  (`|ExecutionSequence`
    (:`then_0`
      ;[1 1 1] Get Reference to rotation helper
      (bind _returnvalue (`entity_base.FindActorByName` "ballRotationHelper" self))
      (bind _asentity_launcher_bp (cast `/Game/blueprint/entity_launcher_BP` _returnvalue))
      (set `self.rotationHelper` _asentity_launcher_bp))
    (:`then_1`
      ;[1 1 1] Get Reference to autoaim launcher
      (bind _returnvalue_2 (`entity_base.FindActorByName` "autoaim" self))
      (bind _asentity_launcher_bp_2 (cast `/Game/blueprint/entity_launcher_BP` _returnvalue_2))
      (set `self.autoaim` _asentity_launcher_bp_2))))

(event `self.ReceiveActorBeginOverlap`
  (params (OtherActor :type "Actor Object Reference"))
  (`|ExecutionSequence`
    (:`then_0`
      ;[1 1 1] Play Rolling Sound
      (bind _asbp_pickup_sphere (cast `/Game/blueprint/BP_Pickup_Sphere` OtherActor))
      (bind _output_get (set `self.bowlingBall` _asbp_pickup_sphere))
      (`GameplayStatics.SpawnSoundAttached` "/Game/sound/Bowling_Ball_Rolling_Sounds_Cue.Bowling_Ball_Rolling_Sounds_Cue" (`entity_base.EntityModel` _asbp_pickup_sphere)))
    (:`then_1`
      ;[1 1 1] Set ball rotation boolean
      (set `self.bRotateBall` true)
      (bind _returnvalue (/ 1500.0 (`KismetMathLibrary.VSize` (`self.GetVelocity` _output_get))))
      ;[1 1 1] Stop ball rotation
      (`KismetSystemLibrary.K2_SetTimerDelegate` (delegate `EndRotation`) _returnvalue)
      ;[1 1 1] Slow Motion
      (`KismetSystemLibrary.K2_SetTimerDelegate` (delegate `DilateTime`) (- _returnvalue 0.75)))
    (:`then_2`
      ;[1 1 1] Reset rotation speed
      (set `entity_launcher.angularLaunchSpeed` (0.0 0.0 0.0) (`self.rotationHelper`)))))

(event `EndRotation`
  ;[1 1 1] Stop ball rotation
  (set `self.bRotateBall` false))

(event `DilateTime`
  ;[1 1 1] Slow Motion
  (`GameplayStatics.SetGlobalTimeDilation` 0.1)
  (`KismetSystemLibrary.K2_SetTimerDelegate` (delegate `UndilateTime`) 0.75))

(event `UndilateTime`
  ;[1 1 1] Slow Motion
  (`GameplayStatics.SetGlobalTimeDilation` 1.0))

(event `self.ReceiveTick`
  (params (DeltaSeconds :type "Float (single-precision)"))
  (`|ExecutionSequence`
    (:`then_0`
      ;[1 1 1] Check if we're rotating
      (if (`self.bRotateBall`)
        (`|ExecutionSequence`
          (:`then_0`
            ;[1 1 1] Call for rotation
            (`entity_launcher.launchProjectileAngular` (`self.rotationHelper`) false false))
          (:`then_1`
            ;[1 1 1] Calculate new rotation speed based on distance
            (bind _returnvalue (`info_target.FindTargetByName` (`self.highestVelocityPoint`) self))
            (bind _returnvalue_2 (`info_target.GetOffsetToActor` _returnvalue (`self.bowlingBall`)))
            (set `entity_launcher.angularLaunchSpeed` (`KismetMathLibrary.MakeVector` 0.0 (`KismetMathLibrary.Square` (/ (- 1700.0 (`KismetMathLibrary.VSize` _returnvalue_2)) 50.0))) (`self.rotationHelper`))))))))

(fn `UserConstructionScript`)