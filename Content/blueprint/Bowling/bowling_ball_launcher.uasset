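; Bowling ball launcher actor that teleports a ball to its own location and fires it with a set linear velocity and spin.
; On BeginPlay it finds the tagged Trigger_Throw and a tagged BP_Pickup_Sphere as the first target, then launches that sphere immediately.
; LaunchLatestBall repeats the launch on the ball returned by the throw trigger's GetBowlingBall.
; Launching overwrites physics velocities on the ball's EntityModel.
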(event `self.ReceiveBeginPlay`
  (`|ExecutionSequence`
    (:`then_0`
      ;[1 1 1] Set Trigger_Throw
      (bind _results (`JavascriptLibrary.GetObjectsOfClass` "/Game/blueprint/Bowling/Trigger_Throw.Trigger_Throw_C" true))
      (for _array_element _results
        (bind _astrigger_throw (cast `/Game/blueprint/Bowling/Trigger_Throw` _array_element))
        (if (`self.ActorHasTag` _astrigger_throw "Trigger_Throw")
          (set `self.Trigger_Throw` _astrigger_throw))))
    (:`then_1`
      ;[1 1 1] Set initial launch target
      (bind _results_2 (`JavascriptLibrary.GetObjectsOfClass` "/Game/blueprint/BP_Pickup_Sphere.BP_Pickup_Sphere_C" true))
      (for _array_element_2 _results_2
        (bind _asbp_pickup_sphere (cast `/Game/blueprint/BP_Pickup_Sphere` _array_element_2))
        (if (`self.ActorHasTag` _asbp_pickup_sphere "BP_Pickup_Sphere")
          (set `self.launchTarget` _asbp_pickup_sphere))))
    (:`then_2`
      (`self.LaunchBall`))))

(fn `LaunchBall`
  (bind _entitymodel (`entity_base.EntityModel` (`self.launchTarget`)))
  ;[1 1 1] Teleport to self
  (`self.K2_SetActorLocation` (`self.launchTarget`) (`self.K2_GetActorLocation` self) false true)
  ;[1 1 1] Launch the ball
  (`PrimitiveComponent.SetPhysicsAngularVelocity` _entitymodel (0.0 0.0 0.0) false "None")
  (`PrimitiveComponent.SetPhysicsLinearVelocity` _entitymodel (`self.LaunchVelocity`) false "None")
  (`self.SpinBall`))

(fn `LaunchLatestBall`
  (bind _entitymodel (`entity_base.EntityModel` (`self.launchTarget`)))
  (bind _bowlingball (`/Game/blueprint/Bowling/Trigger_Throw.GetBowlingBall` (`self.Trigger_Throw`)))
  ;[1 1 1] Teleport to self
  (bind _output_get (set `self.launchTarget` _bowlingball))
  (`self.K2_SetActorLocation` _output_get (`self.K2_GetActorLocation` self) false true)
  ;[1 1 1] Launch the ball
  (`PrimitiveComponent.SetPhysicsAngularVelocity` _entitymodel (0.0 0.0 0.0) false "None")
  (`PrimitiveComponent.SetPhysicsLinearVelocity` _entitymodel (`self.LaunchVelocity`) false "None")
  (`self.SpinBall`))

(fn `SpinBall`
  (`PrimitiveComponent.SetPhysicsAngularVelocity` (`entity_base.EntityModel` (`self.launchTarget`)) (`self.SpinVelocity`) false "None"))

(fn `UserConstructionScript`)