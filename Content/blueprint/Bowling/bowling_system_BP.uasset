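; Bowling game system Blueprint that resets the game and pins on BeginPlay and handles the high score board at game over.
; OnGameover appends the player's name and absolute score from frame index 9 as a new score entry.
; It then loads the score table, formats each entry in place, reveals the 3D HighScoreTable widget on ScoreScreen and passes it the table.
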(event `self.ReceiveBeginPlay`
  (`self.ResetGame`)
  (`self.ResetAndLowerAllPins`))

(event `self.OnGameover`
  (bind _scoretable (`self.scoreTable`))
  (bind _highscoretable (`/Game/blueprint/Bowling/3D_bowling_highscoretable.HighScoreTable` (`self.ScoreScreen`)))
  ;[1 1 1] Append new score
  (`self.appendNewScore` (`KismetStringLibrary.Conv_StringToInt` (`self.GetStringScoreOfFrame` 9 "AbsoluteScore")) (`self.playerName`))
  ;[1 1 1] Print out new score to 3D widget
  (`self.loadScoreTable` _scoretable)
  (for (_array_element _array_index) _scoretable
    (bind _returnvalue (`self.formatScoreString` _array_element))
    (`KismetArrayLibrary.Array_Set` _scoretable _array_index _returnvalue))
  (`SceneComponent.SetVisibility` _highscoretable true true)
  (bind _asbowling_highscoretable (cast `/Game/blueprint/Bowling/bowling_highscoretable` (`WidgetComponent.GetUserWidgetObject` _highscoretable)))
  (`/Game/blueprint/Bowling/bowling_highscoretable.UpdateScoreTable` _asbowling_highscoretable (`self.scoreTable`)))

(fn `UserConstructionScript`)