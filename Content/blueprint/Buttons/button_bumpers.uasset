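; Button Blueprint that raises or retracts lane bumpers by toggling linear-mover props when pressed.
; On BeginPlay it gathers every Prop_movelinear_BP tagged "bumper" into an array.
; OnPressed calls Toggle on each cached bumper, so one button switches all of them without per-instance references.
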(event `self.ReceiveBeginPlay`
  (`|ExecutionSequence`
    (:`then_0`
      ;[1 1 1] Get Lane Bumpers
      (bind _results (`JavascriptLibrary.GetObjectsOfClass` "/Game/blueprint/prop_movelinear_BP.prop_movelinear_BP_C"))
      (for _array_element _results
        (bind _asprop_movelinear_bp (cast `/Game/blueprint/prop_movelinear_BP` _array_element))
        (if (`self.ActorHasTag` _asprop_movelinear_bp "bumper")
          (`KismetArrayLibrary.Array_Add` (`self.Bumper`) _asprop_movelinear_bp))))))

(event `self.OnPressed`
  ;[1 1 1] Toggle Lane Bumpers
  (for _array_element (`self.Bumper`)
    (`self.Toggle` _array_element)))

(fn `UserConstructionScript`)