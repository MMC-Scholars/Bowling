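; Trigger volume that processes each bowling throw after an actor overlaps it and a short timer delay expires.
; It finds the tagged bowling system at BeginPlay, then on each throw has it calculate the score and writes that to every score board's text render.
; It then resets the tagged ball's transform and has the system reset the pins, checking whether it awaits a first throw.
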(event `self.ReceiveBeginPlay`
  (`|ExecutionSequence`
    (:`then_0`
      ;[1 1 1] Set Bowling System
      (bind _results (`JavascriptLibrary.GetObjectsOfClass` "/Script/MMC_Bowling.bowling_system" true))
      (for _array_element _results
        (bind _asbowling_system_bp (cast `/Game/blueprint/bowling_system_BP` _array_element))
        (if (`self.ActorHasTag` _asbowling_system_bp "bowling_system_BP")
          (set `self.Bowling_System` _asbowling_system_bp))))))

(event `self.ReceiveActorBeginOverlap`
  (params (OtherActor :type "Actor Object Reference"))
  (`KismetSystemLibrary.K2_SetTimerDelegate` (delegate `ProcessThrow`) (`self.ProcessThrowDelay`)))

(event `ProcessThrow`
  (bind _bowling_system (`self.Bowling_System`))
  (bind _bowling_system_2 (`self.Bowling_System`))
  (`|ExecutionSequence`
    (:`then_0`
      ;[1 1 1] Set Bowling Ball
      (if (`self.ActorHasTag` (stale `self.ReceiveActorBeginOverlap` OtherActor) "bowling_ball")
        (bind _asbp_pickup_sphere (cast `/Game/blueprint/BP_Pickup_Sphere` (stale `self.ReceiveActorBeginOverlap` OtherActor)))
        (set `self.Bowling_Ball` _asbp_pickup_sphere)))
    (:`then_1`
      ;[1 1 1] Calculate Score
      (`bowling_system.CalculateScore` _bowling_system)
      ;[1 1 1] Print Score
      (bind _returnvalue (`bowling_system.GetStringScoreOfGame` _bowling_system))
      (bind _results (`JavascriptLibrary.GetObjectsOfClass` "/Game/blueprint/bowling_score_BP.bowling_score_BP_C" true))
      (for _array_element _results
        (bind _asbowling_score_bp (cast `/Game/blueprint/bowling_score_BP` _array_element))
        (`TextRenderComponent.K2_SetText` (`TextRenderActor.TextRender` _asbowling_score_bp) (`KismetTextLibrary.Conv_StringToText` _returnvalue))))
    (:`then_2`
      ;[1 1 1] Reset Bowling Ball
      (`entity_base.ResetWorldTransform` (`self.Bowling_Ball`)))
    (:`then_3`
      ;[1 1 1] Reset Pins As Necessary
      (`bowling_system.WaitingForFirstThrow` _bowling_system_2)
      (if true
        (`bowling_system.ResetAndLowerAllPins` _bowling_system_2)
        (else
          (`bowling_system.RaiseAndLowerUnfallenPins` _bowling_system_2))))))

(fn `UserConstructionScript`)