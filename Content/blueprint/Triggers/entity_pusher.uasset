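; Trigger actor that pushes overlapping entity_base actors along a preset direction, like a current or conveyor zone.
; Overlap begin and end events maintain an array of affected entities.
; Tick counts frames and periodically fires PushActors, which blends each entity's velocity toward direction times push speed and applies it to the EntityModel's physics linear velocity.
; The push direction is made unit length by clamping the vector's size to about one.
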(event `self.ReceiveBeginPlay`)

(event `self.ReceiveActorBeginOverlap`
  (params (OtherActor :type "Actor Object Reference"))
  ;[1 1 1] Add/Remove effected entities with array
  (bind _asentity_base (cast `entity_base` OtherActor))
  (`KismetArrayLibrary.Array_AddUnique` (`self.PushedEntities`) _asentity_base))

(event `self.ReceiveActorEndOverlap`
  (params (OtherActor :type "Actor Object Reference"))
  ;[1 1 1] Add/Remove effected entities with array
  (bind _asentity_base (cast `entity_base` OtherActor))
  (`KismetArrayLibrary.Array_RemoveItem` (`self.PushedEntities`) _asentity_base))

(event `self.ReceiveTick`
  (params (DeltaSeconds :type "Float (single-precision)"))
  ;[1 1 1] Push actors only after so many ticks
  (bind _output_get (set `self.TickCount` (+ (`self.TickCount`) 1)))
  (if (>= _output_get (`self.MaxTickCount`))
    (set `self.TickCount` 0)
    (`self.PushActors`)))

(event `PushActors`
  ;[1 1 1] Push Actors Event
  (for _array_element (`self.PushedEntities`)
    (bind _unitdirection (`self.GetPushDirectionUnit`))
    (`PrimitiveComponent.SetPhysicsLinearVelocity` (`entity_base.EntityModel` _array_element) (`KismetMathLibrary.VLerp` (`self.GetVelocity` _array_element) (* _unitdirection (`self.PushSpeed`)) (`self.Lerp`)) false "None")))

(fn `GetPushDirectionUnit`
  (returns (UnitDirection :type "Vector Structure"))
  ;[1 1 1] Return pre-defined direction
  (return (`KismetMathLibrary.ClampVectorSize` (`self.PushDirection`) 0.999 1.001)))

(fn `UserConstructionScript`)