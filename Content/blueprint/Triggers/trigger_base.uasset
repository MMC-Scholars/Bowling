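; Base trigger actor that tracks overlapping actors and passes overlaps to empty BeginOverlap and EndOverlap hooks for child Blueprints.
; On BeginPlay it looks up an optional filter_base_BP by name, whose FilterActor gates entries.
; A Tick-driven cooldown limits BeginOverlap calls, though accepted actors are still recorded during it.
; EndOverlap fires only for recorded actors, and helpers query or clear the list.
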(event `self.ReceiveBeginPlay`
  ;[1 1 1] Get Reference to filter
  (bind _returnvalue (`entity_base.FindActorByName` (`self.Filter Name`) self))
  (bind _asfilter_base_bp (cast `/Game/blueprint/Triggers/filter_base_BP` _returnvalue)
    (:`then`
      (set `self.Filter` _asfilter_base_bp)
      ;[1 1 1] Remember if we found it or not
      (set `self.bNoFilter` false))
    (:`CastFailed`
      (set `self.bNoFilter` true))))

(event `self.ReceiveActorBeginOverlap`
  (params (OtherActor :type "Actor Object Reference"))
  ;[1 1 1] Check if we do anything on overlap
  (if (`self.bNoFilter`)
    ;[1 1 1] Add to overlapping actor array
    (`KismetArrayLibrary.Array_AddUnique` (`self.OverlappingActors`) OtherActor :!label _label)
    ;[1 1 1] Check if we're after the delay before reset
    (if (> (`self.DelayWaitingTime`) (`self.Delay before reset`))
      ;[1 1 1] Call Implemenatble Function
      (`self.BeginOverlap` OtherActor)
      ;[1 1 1] Reset delay waiting time
      (set `self.DelayWaitingTime` 0.0))
    (elif (`filter_base.FilterActor` (`self.Filter`) OtherActor)
      (goto _label))))

(event `self.ReceiveActorEndOverlap`
  (params (OtherActor :type "Actor Object Reference"))
  ;[1 1 1] Remove from array, always
  (bind _returnvalue (`KismetArrayLibrary.Array_RemoveItem` (`self.OverlappingActors`) OtherActor))
  (if _returnvalue
    (`self.EndOverlap` OtherActor)))

(event `self.ReceiveTick`
  (params (DeltaSeconds :type "Float (single-precision)"))
  ;[1 1 1] Increment the waiting time
  (set `self.DelayWaitingTime` (+ DeltaSeconds (`self.DelayWaitingTime`))))

(fn `ActorIsOverlapping`
  (params (TestedActor :type "Actor Object Reference"))
  (returns (ActorIsOverlapping :type Boolean))
  (return (`KismetArrayLibrary.Array_Contains` (`self.OverlappingActors`) TestedActor)))

(fn `BeginOverlap`
  (params (InActor :type "Actor Object Reference")))

(fn `ClearOverlapList`
  (`KismetArrayLibrary.Array_Clear` (`self.OverlappingActors`)))

(fn `EndOverlap`
  (params (OutActor :type "Actor Object Reference")))

(fn `UserConstructionScript`)