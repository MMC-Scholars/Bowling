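; Trigger Blueprint for teleporting that resolves its destination by TargetName on BeginPlay, accepting either an entity_launcher_BP or an info_target.
; With a launcher, BeginOverlap sets the overlapping actor as its projectile by name and launches it with teleport-before-launch enabled.
; With an info_target, it stores the target and sets IsTarget; this graph takes no further action on overlap.
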(event `self.ReceiveBeginPlay`
  ;[1 1 1] Don't change these; use the implementable functions instead
  (`parent.ReceiveBeginPlay`)
  ;[1 1 1] Get reference to teleport target
  (bind _returnvalue (`entity_base.FindActorByName` (`self.TargetName`) self))
  (bind _asentity_launcher_bp (cast `/Game/blueprint/entity_launcher_BP` _returnvalue)
    (:`then`
      (set `self.Launcher` _asentity_launcher_bp)
      (set `self.bIsTarget` false))
    (:`CastFailed`
      (bind _asinfo_target (cast `info_target` _returnvalue))
      (set `self.Target` _asinfo_target)
      (set `self.bIsTarget` true))))

(event `self.ReceiveActorBeginOverlap`
  (params (OtherActor :type "Actor Object Reference"))
  ;[1 1 1] Don't change these; use the implementable functions instead
  (`parent.ReceiveActorBeginOverlap` OtherActor))

(event `self.ReceiveTick`
  (params (DeltaSeconds :type "Float (single-precision)"))
  (`parent.ReceiveTick` DeltaSeconds))

(event `self.BeginOverlap`
  (params (InActor :type "Actor Object Reference"))
  (if (not (`self.bIsTarget`))
    ;[1 1 1] Use the launcher
    (bind _returnvalue (`JavascriptLibrary.GetName` InActor))
    (`entity_launcher.setProjectile` (`self.Launcher`) (`KismetStringLibrary.Conv_StringToName` _returnvalue))
    (`entity_launcher.launchProjectile` (`self.Launcher`) true false)))

(fn `UserConstructionScript`
  (`parent.UserConstructionScript`))