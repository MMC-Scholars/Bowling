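; A world-space virtual keyboard Blueprint for entering the bowling player's name with VR motion controllers.
; Overlapping the box with a motion controller feeds a point just ahead of the controller to AppendFromTargetLocation and plays a sound.
; Text changes update the copied string and switch the Paper sprite between capital and lowercase layouts, depending on whether it is empty.
; Enter hides the text, stores the name in the BowlingSystem and flags it ready.
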(event `self.ReceiveBeginPlay`
  (`|ExecutionSequence`
    (:`then_0`
      ;[1 1 1] Reset sprite
      (`PaperSpriteComponent.SetSprite` (`self.PaperSprite`) "/Game/materials/GUI/virtual_keyboard/capital_Sprite.capital_Sprite"))))

(event `self.OnTextChanged`
  (bind _papersprite (`self.PaperSprite`))
  (bind _returnvalue (`KismetTextLibrary.Conv_TextToString` (`TextRenderComponent.Text` (`self.TextRender`))))
  ;[1 1 1] Switch between capital and lowercase sprites
  (set `self.textCopy` _returnvalue)
  (if (and (== (`KismetStringLibrary.Len` _returnvalue) 0) (!= _papersprite null))
    (`PaperSpriteComponent.SetSprite` _papersprite "/Game/materials/GUI/virtual_keyboard/capital_Sprite.capital_Sprite")
    (else
      (`PaperSpriteComponent.SetSprite` _papersprite "/Game/materials/GUI/virtual_keyboard/lower_Sprite.lower_Sprite"))))

(event `DetectTargetInput`
  (params (HitResult :type "HitResult Structure"))
  ;[1 1 1] Receive input from any received hit result
  (`self.AppendFromTargetLocation` HitResult_Location (`self.textCopy`))
  (`AudioComponent.Play` (`self.Audio`) 0.0))

(event `self.OnEnter`
  ;[1 1 1] End input on enter
  (`SceneComponent.SetVisibility` (`self.TextRender`) false true)
  (set `/Game/blueprint/Bowling/bowling_system_BP.playerName` (`KismetStringLibrary.Conv_StringToName` (`self.textCopy`)) (`self.bowlingSystem`))
  (set `self.nameIsReady` true))

(event `self.Box.OnComponentBeginOverlap`
  (params (OverlappedComponent :type "PrimitiveComponent Object Reference") (OtherActor :type "Actor Object Reference") (OtherComp :type "PrimitiveComponent Object Reference") (OtherBodyIndex :type Integer) (bFromSweep :type Boolean) (SweepResult :type "HitResult Structure (by ref)"))
  ;[1 1 1] Detect Motion Controller Overlap for Input
  (bind _asbp_motion_controller (cast `/Game/VirtualRealityBP/Blueprints/BP_MotionController` OtherActor))
  (bind _motioncontroller (`/Game/VirtualRealityBP/Blueprints/BP_MotionController.MotionController` _asbp_motion_controller))
  (`self.DetectTargetInput` (`GameplayStatics.MakeHitResult` false false 0.0 (+ (`SceneComponent.K2_GetComponentLocation` _motioncontroller) (`KismetMathLibrary.GreaterGreater_VectorRotator` (`KismetMathLibrary.MakeVector` 3.0) (`SceneComponent.RelativeRotation` _motioncontroller))))))

(fn `UserConstructionScript`)